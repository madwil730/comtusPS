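; BP_Lock is an interactable lock puzzle with three cubes, shown in an inspect view.
; Interacting spawns a distant BP_InspectItem hosting BP_LockUI, adds W_Inspect and moves input from pawn to lock; IA_Interact reverses this.
; A and D step an enum selection, marked by an outline overlay material.
; W starts a Tick-driven rotation lerp that looks unfinished: it only handles Cube 1, rotates Cube2 instead and never stops.
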(event `/Game/Lee/BP/Inspect/InteractInterface.Interacted`
  (params (Character :type "/Game/ThirdPerson/Blueprints/BP_FirstPersonCharacter Object Reference"))
  (bind _returnvalue (`GameplayStatics.GetPlayerController` 0))
  (bind _childactor (`/Game/Lee/BP/Inspect/BP_InspectItem.childActor` (`self.InspectUI`)))
  (bind _returnvalue_2 (`|SpawnActorFromClass` "/Game/Lee/BP/Inspect/BP_InspectItem.BP_InspectItem_C" (`KismetMathLibrary.MakeTransform` (1000000.0 0.0 0.0)) "Undefined" "MultiplyWithRoot" null null))
  (bind _output_get (set `self.InspectUI` _returnvalue_2))
  (`/Game/Lee/BP/Inspect/BP_InspectItem.set Inspect Rotation` :`self` _output_get)
  (`/Game/Lee/BP/Inspect/BP_InspectItem.Set Inspect Scale` _output_get (1.0 1.0 1.0))
  (bind _returnvalue_3 (`|CreateWidget` "/Game/Lee/UI/Inspect/W_Inspect.W_Inspect_C"))
  (bind _output_get_2 (set `self.InspectWidgetRef` _returnvalue_3))
  (`UserWidget.AddToViewport` _output_get_2 0)
  (`self.DisableInput` (`GameplayStatics.GetPlayerPawn` 0) _returnvalue)
  (`self.EnableInput` _returnvalue)
  (`ChildActorComponent.SetChildActorClass` _childactor "/Game/Lee/BP/Puzzle/BP_LockUI.BP_LockUI_C")
  (bind _asbp_lock_ui (cast `/Game/Lee/BP/Puzzle/BP_LockUI` (`ChildActorComponent.ChildActor` _childactor)))
  (bind _output_get_3 (set `self.BP Lock UI` _asbp_lock_ui))
  (`MeshComponent.SetOverlayMaterial` (`/Game/Lee/BP/Puzzle/BP_LockUI.Cube1` _output_get_3) "/Game/Lee/BP/Puzzle/M_Outline.M_Outline"))

(event `EnhancedInput|/Game/ThirdPerson/Input/Actions/IA_Interact`
  (params (ActionValue :type Boolean) (ElapsedSeconds :type "Float (double-precision)") (TriggeredSeconds :type "Float (double-precision)") (InputAction :type "InputAction Object Reference" :default "/Game/ThirdPerson/Input/Actions/IA_Interact.IA_Interact"))
  (bind _returnvalue (`GameplayStatics.GetPlayerController` 0))
  (bind _inspectwidgetref (`self.InspectWidgetRef`))
  (:`Started`
    (`self.DisableInput` _returnvalue)
    (`self.EnableInput` (`GameplayStatics.GetPlayerPawn` 0) _returnvalue)
    (`/Engine/EditorBlueprintResources/StandardMacros.IsValid` _inspectwidgetref
      (:`Is Valid`
        (`Widget.RemoveFromParent` _inspectwidgetref)
        (`self.K2_DestroyActor` (`self.InspectUI`))))))

(event `Key|D`
  (params (Key :type "Key Structure"))
  (bind _bp_lock_ui (`self.BP Lock UI`))
  (bind _bp_lock_ui_2 (`self.BP Lock UI`))
  (:`Pressed`
    (switch `/Game/Lee/BP/Puzzle/LockEnum` (`self.LockEnum`)
      (:`NewEnumerator0`
        (set `self.LockEnum` "NewEnumerator1")
        (`MeshComponent.SetOverlayMaterial` (`/Game/Lee/BP/Puzzle/BP_LockUI.Cube2` _bp_lock_ui) "/Game/Lee/BP/Puzzle/M_Outline.M_Outline")
        (`MeshComponent.SetOverlayMaterial` (`/Game/Lee/BP/Puzzle/BP_LockUI.Cube1` _bp_lock_ui) null))
      (:`NewEnumerator1`
        (set `self.LockEnum` "NewEnumerator2")
        (`MeshComponent.SetOverlayMaterial` (`/Game/Lee/BP/Puzzle/BP_LockUI.Cube3` _bp_lock_ui_2) "/Game/Lee/BP/Puzzle/M_Outline.M_Outline")
        (`MeshComponent.SetOverlayMaterial` (`/Game/Lee/BP/Puzzle/BP_LockUI.Cube2` _bp_lock_ui_2) null)))))

(event `Key|A`
  (params (Key :type "Key Structure"))
  (bind _bp_lock_ui (`self.BP Lock UI`))
  (bind _bp_lock_ui_2 (`self.BP Lock UI`))
  (:`Pressed`
    (switch `/Game/Lee/BP/Puzzle/LockEnum` (`self.LockEnum`)
      (:`NewEnumerator1`
        (set `self.LockEnum` "NewEnumerator0")
        (`MeshComponent.SetOverlayMaterial` (`/Game/Lee/BP/Puzzle/BP_LockUI.Cube1` _bp_lock_ui) "/Game/Lee/BP/Puzzle/M_Outline.M_Outline")
        (`MeshComponent.SetOverlayMaterial` (`/Game/Lee/BP/Puzzle/BP_LockUI.Cube2` _bp_lock_ui) null))
      (:`NewEnumerator2`
        (set `self.LockEnum` "NewEnumerator1")
        (`MeshComponent.SetOverlayMaterial` (`/Game/Lee/BP/Puzzle/BP_LockUI.Cube2` _bp_lock_ui_2) "/Game/Lee/BP/Puzzle/M_Outline.M_Outline")
        (`MeshComponent.SetOverlayMaterial` (`/Game/Lee/BP/Puzzle/BP_LockUI.Cube3` _bp_lock_ui_2) null)))))

(event `Key|W`
  (params (Key :type "Key Structure"))
  (:`Pressed`
    (set `self.IsMoving ` true)))

(event `self.ReceiveTick`
  (params (DeltaSeconds :type "Float (single-precision)"))
  (bind _cube2 (`/Game/Lee/BP/Puzzle/BP_LockUI.Cube2` (`self.BP Lock UI`)))
  (if (`self.IsMoving `)
    (set `self.ElapsedTime ` 0.0)
    (switch `/Game/Lee/BP/Puzzle/LockEnum` (`self.LockEnum`)
      (:`NewEnumerator0`
        (`SceneComponent.K2_SetRelativeRotation` _cube2 (`KismetMathLibrary.RLerp` (`SceneComponent.RelativeRotation` _cube2) (`KismetMathLibrary.MakeRotator` 90.0) (* DeltaSeconds 2.0)) false false)))))

(fn `UserConstructionScript`)