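; BP_Talisman is an interactable puzzle where the player hides five cubes in a required order.
; Interacting blends the view to the actor and moves input from the pawn to it until IA_Interact returns both.
; W/S move an outline overlay through the cube array; F hides the selected cube and checks it against CorrectOrder.
; Tick calls the HUD widget's FailEvent after five picks if any was wrong; success is not handled.
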(event `self.ReceiveBeginPlay`
  (`self.Set Item`))

(event `/Game/Lee/BP/Inspect/InteractInterface.Interacted`
  (params (Character :type "/Game/ThirdPerson/Blueprints/BP_FirstPersonCharacter Object Reference"))
  (bind _returnvalue (`GameplayStatics.GetPlayerController` 0))
  (`self.DisableInput` (`GameplayStatics.GetPlayerPawn` 0) _returnvalue)
  (`self.EnableInput` _returnvalue)
  (`PlayerController.SetViewTargetWithBlend` (`GameplayStatics.GetPlayerController` 0) self 1.0 "VTBlend_Linear" 0.0 false)
  (`MeshComponent.SetOverlayMaterial` (`self.Cube1`) "/Game/Lee/BP/Puzzle/M_Outline.M_Outline"))

(event `EnhancedInput|/Game/ThirdPerson/Input/Actions/IA_Interact`
  (params (ActionValue :type Boolean) (ElapsedSeconds :type "Float (double-precision)") (TriggeredSeconds :type "Float (double-precision)") (InputAction :type "InputAction Object Reference" :default "/Game/ThirdPerson/Input/Actions/IA_Interact.IA_Interact"))
  (bind _returnvalue (`GameplayStatics.GetPlayerController` 0))
  (:`Started`
    (`self.DisableInput` _returnvalue)
    (`self.EnableInput` (`GameplayStatics.GetPlayerPawn` 0) _returnvalue)
    (`PlayerController.SetViewTargetWithBlend` (`GameplayStatics.GetPlayerController` 0) (`GameplayStatics.GetPlayerPawn` 0) 1.0 "VTBlend_Linear" 0.0 false)))

(event `Key|W`
  (params (Key :type "Key Structure"))
  (bind _index (`self.Index`))
  (:`Pressed`
    (if (> _index 0)
      (`MeshComponent.SetOverlayMaterial` (`|GetArrayItem` (`self.staticMesh`) (`self.Index`)) null)
      (`/Engine/EditorBlueprintResources/StandardMacros.DecrementInt` _index
        (:`  `
          (`MeshComponent.SetOverlayMaterial` (`|GetArrayItem` (`self.staticMesh`) (`self.Index`)) "/Game/Lee/BP/Puzzle/M_Outline.M_Outline"))))))

(event `Key|S`
  (params (Key :type "Key Structure"))
  (bind _index (`self.Index`))
  (:`Pressed`
    (bind _result (`/Engine/EditorBlueprintResources/StandardMacros.DecrementInt` (`KismetArrayLibrary.Array_Length` (`self.staticMesh`)))
      (:`  `
        (if (< _index _result)
          (`MeshComponent.SetOverlayMaterial` (`|GetArrayItem` (`self.staticMesh`) (`self.Index`)) null)
          (`/Engine/EditorBlueprintResources/StandardMacros.IncrementInt` _index
            (:`  `
              (`MeshComponent.SetOverlayMaterial` (`|GetArrayItem` (`self.staticMesh`) (`self.Index`)) "/Game/Lee/BP/Puzzle/M_Outline.M_Outline"))))))))

(event `Key|F`
  (params (Key :type "Key Structure"))
  (bind _index (`self.Index`))
  (:`Pressed`
    (`KismetSystemLibrary.PrintString` (`KismetStringLibrary.Conv_IntToString` _index))
    (`SceneComponent.SetVisibility` (`|GetArrayItem` (`self.staticMesh`) _index) false false)
    (if (not (== (`|GetArrayItem` (`self.CorrectOrder`) (`self.CurrentIndex`)) (`self.Index`)))
      (set `self.FailCheck` true))
    (`KismetSystemLibrary.PrintString` (`KismetStringLibrary.Conv_BoolToString` (`self.FailCheck`)))
    (`/Engine/EditorBlueprintResources/StandardMacros.IncrementInt` (`self.CurrentIndex`))))

(event `self.ReceiveTick`
  (params (DeltaSeconds :type "Float (single-precision)"))
  (if (> (`self.CurrentIndex`) 4)
    (if (`self.FailCheck`)
      (set `self.FailCheck` false)
      (bind _asmy_hud (cast `/Game/Lee/GameMode/MyHUD` (`PlayerController.GetHUD` (`GameplayStatics.GetPlayerController` 0))))
      (bind _wplayerui (`/Game/Lee/GameMode/MyHUD.WPlayerUI` _asmy_hud))
      (`/Engine/EditorBlueprintResources/StandardMacros.IsValid` _wplayerui
        (:`Is Valid`
          (`/Game/Lee/UI/W_PlayerUI.FailEvent` _wplayerui))))))

(fn `Set Item`
  (bind _staticmesh (`self.staticMesh`))
  (`KismetArrayLibrary.Array_Add` _staticmesh (`self.Cube1`))
  (`KismetArrayLibrary.Array_Add` _staticmesh (`self.Cube2`))
  (`KismetArrayLibrary.Array_Add` _staticmesh (`self.Cube3`))
  (`KismetArrayLibrary.Array_Add` _staticmesh (`self.Cube4`))
  (`KismetArrayLibrary.Array_Add` _staticmesh (`self.Cube5`)))

(fn `UserConstructionScript`)