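; Interactive door that the player cycles through closed, partially open and fully open, swinging according to the side they face.
; Tick polls the player's interact flag and hit actor; a dot product sets the swing sign and a timer advances the state.
; While interaction holds, HandleDoor picks the state's target angle and steps rotation with FInterpTo.
; Leaving the box triggers a delayed, single closing step, depending on player facing.
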(event `self.ReceiveBeginPlay`
  (bind _asbp_first_person_character (cast `/Game/ThirdPerson/Blueprints/BP_FirstPersonCharacter` (`GameplayStatics.GetPlayerCharacter` 0)))
  (set `self.CharacterRef` _asbp_first_person_character))

(event `self.ReceiveTick`
  (params (DeltaSeconds :type "Float (single-precision)"))
  (bind _characterref (`self.CharacterRef`))
  (if (and (`/Game/ThirdPerson/Blueprints/BP_FirstPersonCharacter.IsInteracting?` _characterref) (== (`/Game/ThirdPerson/Blueprints/BP_FirstPersonCharacter.Hit Actor` _characterref) self))
    (if (`self.bisInteractDoor`)
      (`self.HandleDoor`)
      (else
        (`self.IsInteractWithDoor` (`self.CharacterRef`))))))

(event `IsInteractWithDoor`
  (params (Player :type "/Game/ThirdPerson/Blueprints/BP_FirstPersonCharacter Object Reference"))
  ;[1 1 1] Door Interact
  (if (> (`KismetMathLibrary.Dot_VectorVector` (`self.GetActorForwardVector` Player) (`SceneComponent.GetForwardVector` (`self.DoorOpenLocation`))) 0.0)
    (set `self.Door Open Side` 1.0)
    (else
      (set `self.Door Open Side` -1.0)))
  (set `self.bisInteractDoor` true)
  (`KismetSystemLibrary.K2_SetTimerDelegate` (delegate `CustomEvent`) (`self.Door Sound Time`)))

(event `CustomEvent`
  ;[1 1 1] Door Interact
  (set `self.bisInteractDoor` false)
  (switch `/Game/Lee/Enum/E_DoorState` (`self.EDoorState`)
    (:`NewEnumerator0`
      (set `self.EDoorState` "NewEnumerator1"))
    (:`NewEnumerator1`
      (set `self.EDoorState` "NewEnumerator2"))
    (:`NewEnumerator2`
      (set `self.EDoorState` "NewEnumerator0"))))

(event `self.Box.OnComponentEndOverlap`
  (params (OverlappedComponent :type "PrimitiveComponent Object Reference") (OtherActor :type "Actor Object Reference") (OtherComp :type "PrimitiveComponent Object Reference") (OtherBodyIndex :type Integer))
  (bind _returnvalue (`GameplayStatics.GetPlayerCharacter` 0))
  (bind (_returnvalue_x _returnvalue_y) (`KismetMathLibrary.BreakVector` (`self.GetActorForwardVector` _returnvalue)))
  ;[1 1 1] Automatic dor close
  (if (and (== OtherActor _returnvalue) (`KismetMathLibrary.BooleanNOR` (>= _returnvalue_y 0.7) (<= _returnvalue_y -0.7)))
    (`KismetSystemLibrary.Delay` 0.5)
    (set `self.bisInteractDoor` true)
    (`self.HandleRoation` 0.0)
    (`KismetSystemLibrary.Delay` 1.4)
    (set `self.bisInteractDoor` false)))

(event `HandleDoor`
  ;[1 1 1] Handle Door
  (switch `/Game/Lee/Enum/E_DoorState` (`self.EDoorState`)
    (:`NewEnumerator0`
      (`self.HandleRoation` (* 15.0 (`self.Door Open Side`))))
    (:`NewEnumerator1`
      (`self.HandleRoation` (* (`self.Door Open Angle`) (`self.Door Open Side`))))
    (:`NewEnumerator2`
      (`self.HandleRoation` 0.0))))

(event `HandleRoation`
  (params (`Set Rotaiton` :type "Float (double-precision)"))
  ;[1 1 1] Handle Rotation
  (`SceneComponent.K2_SetRelativeRotation` (`self.Door`) (`KismetMathLibrary.MakeRotator` (`KismetMathLibrary.FInterpTo` (.yaw (`SceneComponent.RelativeRotation` (`self.Door`))) `Set Rotaiton` (`GameplayStatics.GetWorldDeltaSeconds`) (`self.Interp Speed`))) false false))

(fn `UserConstructionScript`)