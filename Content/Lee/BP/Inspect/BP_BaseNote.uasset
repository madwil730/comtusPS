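; BP_BaseNote is an interactable note that shows the player an outer or inner proximity icon through two overlap spheres.
; The construction script applies the configurable mesh, scale, icon location, sphere radii and debug visibility.
; With AutoRead, interaction toggles a W_Note widget and locks movement and look via a FlipFlop macro.
; Otherwise, Inspect spawns a far-off BP_InspectItem for viewing and reading, while plain pickup only prints a message.
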(event `self.OuterSphere.OnComponentBeginOverlap`
  (params (OverlappedComponent :type "PrimitiveComponent Object Reference") (OtherActor :type "Actor Object Reference") (OtherComp :type "PrimitiveComponent Object Reference") (OtherBodyIndex :type Integer) (bFromSweep :type Boolean) (SweepResult :type "HitResult Structure (by ref)"))
  (if (== OtherActor (`GameplayStatics.GetPlayerCharacter` 0))
    (`SceneComponent.SetVisibility` (`self.OutIcon`) true false)))

(event `self.InnerSphere.OnComponentBeginOverlap`
  (params (OverlappedComponent :type "PrimitiveComponent Object Reference") (OtherActor :type "Actor Object Reference") (OtherComp :type "PrimitiveComponent Object Reference") (OtherBodyIndex :type Integer) (bFromSweep :type Boolean) (SweepResult :type "HitResult Structure (by ref)"))
  (if (== OtherActor (`GameplayStatics.GetPlayerCharacter` 0))
    (`SceneComponent.SetVisibility` (`self.InnerIcon`) true false)
    (`SceneComponent.SetVisibility` (`self.OutIcon`) false false)))

(event `self.InnerSphere.OnComponentEndOverlap`
  (params (OverlappedComponent :type "PrimitiveComponent Object Reference") (OtherActor :type "Actor Object Reference") (OtherComp :type "PrimitiveComponent Object Reference") (OtherBodyIndex :type Integer))
  (if (== (`GameplayStatics.GetPlayerCharacter` 0) OtherActor)
    (`SceneComponent.SetVisibility` (`self.InnerIcon`) false false)
    (`SceneComponent.SetVisibility` (`self.OutIcon`) true false)))

(event `self.OuterSphere.OnComponentEndOverlap`
  (params (OverlappedComponent :type "PrimitiveComponent Object Reference") (OtherActor :type "Actor Object Reference") (OtherComp :type "PrimitiveComponent Object Reference") (OtherBodyIndex :type Integer))
  (if (== OtherActor (`GameplayStatics.GetPlayerCharacter` 0))
    (`SceneComponent.SetVisibility` (`self.OutIcon`) false false)))

(event `self.ReceiveBeginPlay`
  (bind _asbp_first_person_character (cast `/Game/ThirdPerson/Blueprints/BP_FirstPersonCharacter` (`GameplayStatics.GetPlayerCharacter` 0)))
  (set `self.BP Player Ref` _asbp_first_person_character))

(event `/Game/Lee/BP/Inspect/InteractInterface.Interacted`
  (params (Character :type "/Game/ThirdPerson/Blueprints/BP_FirstPersonCharacter Object Reference"))
  (bind _charactermovement (`Character.CharacterMovement` (`GameplayStatics.GetPlayerCharacter` 0)))
  (if (not (`self.AutoRead?`))
    (if (`self.Inspect?`)
      (bind _returnvalue (`|SpawnActorFromClass` "/Game/Lee/BP/Inspect/BP_InspectItem.BP_InspectItem_C" (`KismetMathLibrary.MakeTransform` (1000000.0 0.0 0.0)) "Undefined" "MultiplyWithRoot" null null))
      (`/Game/Lee/BP/Inspect/BP_InspectItem.set Inspect Rotation` _returnvalue (`self.Imte Inspection Rotation`))
      (`/Game/Lee/BP/Inspect/BP_InspectItem.Set Inspect Scale` _returnvalue (`self.Item InspectionScale`))
      (`/Game/Lee/BP/Inspect/BP_InspectItem.Inspect` _returnvalue Character (`StaticMeshComponent.StaticMesh` (`self.StaticMesh`)) (`self.ItemName`) (`self.ItemDesc`))
      (message `/Game/Lee/BP/Inspect/InteractInterface.ReadNote` _returnvalue Character (`self.NoteText`))
      (else
        (`KismetSystemLibrary.PrintString` "Pick up Note" :!label _label)))
    (else
      (bind _isa (`/Engine/EditorBlueprintResources/StandardMacros.FlipFlop`)
        (:`A`
          (set `self.Is A` _isa)
          (bind _returnvalue_2 (`|CreateWidget` "/Game/Lee/UI/Note/W_Note.W_Note_C" null (`self.NoteText`)))
          (bind _output_get (set `self.NoteWidgetRefrence` _returnvalue_2))
          (`UserWidget.AddToViewport` _output_get 0)
          (`CharacterMovementComponent.DisableMovement` (`Character.CharacterMovement` (`GameplayStatics.GetPlayerCharacter` 0)))
          (`Controller.SetIgnoreLookInput` (`GameplayStatics.GetPlayerController` 0) true)
          (`Widget.SetRenderOpacity` (`/Game/Lee/UI/Note/W_Note.NoteCanvasPanel` (`self.NoteWidgetRefrence`)) 1.0)
          (set `self.Is A` false)
          (goto _label))
        (:`B`
          (`Widget.SetRenderOpacity` (`/Game/Lee/UI/Note/W_Note.NoteCanvasPanel` (`self.NoteWidgetRefrence`)) 0.0)
          (`Widget.RemoveFromParent` _returnvalue_2)
          (`CharacterMovementComponent.SetMovementMode` _charactermovement (`CharacterMovementComponent.DefaultLandMovementMode` _charactermovement) 0)
          (`Controller.SetIgnoreLookInput` (`GameplayStatics.GetPlayerController` 0) false)
          (goto _label))))))

(fn `UserConstructionScript`
  (bind _staticmesh (`self.StaticMesh`))
  (`|ExecutionSequence`
    (:`then_0`
      (`SphereComponent.SetSphereRadius` (`self.InnerSphere`) (`self.InnerSphere Radius`) true)
      (`SphereComponent.SetSphereRadius` (`self.OuterSphere`) (`self.OutSphere Radius`) true)
      (`SceneComponent.K2_SetRelativeLocation` (`self.InnerIcon`) (`self.IconLocation`) false false)
      (`SceneComponent.K2_SetRelativeLocation` (`self.OutIcon`) (`self.IconLocation`) false false))
    (:`then_1`
      (`StaticMeshComponent.SetStaticMesh` (`self.StaticMesh`) (`self.ItemMesh`))
      (`SceneComponent.K2_SetWorldTransform` _staticmesh (`KismetMathLibrary.MakeTransform` (`SceneComponent.K2_GetComponentLocation` _staticmesh) (`SceneComponent.K2_GetComponentRotation` _staticmesh) (`self.ItemScale`)) false false))
    (:`then_2`
      (if (`self.Debugging`)
        (`SceneComponent.SetVisibility` (`self.InnerSphere`) true false)
        (`SceneComponent.SetVisibility` (`self.OuterSphere`) true false)
        (else
          (`SceneComponent.SetVisibility` (`self.InnerSphere`) false false)
          (`SceneComponent.SetVisibility` (`self.OuterSphere`) false false))))))