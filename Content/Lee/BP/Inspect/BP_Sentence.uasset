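; BP_Sentence is an inspectable Blueprint that shows a "잠겨 있다" ("It is locked") message on the player's HUD when interacted with.
; The Interacted event casts player 0's HUD to MyHUD, makes the WPlayerUI text block visible and sets the message.
; A short timer follows, apparently bound to SetHidden, which hides the text block again.
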(event `/Game/Lee/BP/Inspect/InteractInterface.Interacted`
  (params (Character :type "/Game/ThirdPerson/Blueprints/BP_FirstPersonCharacter Object Reference"))
  (bind _asmy_hud (cast `/Game/Lee/GameMode/MyHUD` (`PlayerController.GetHUD` (`GameplayStatics.GetPlayerController` 0))))
  (bind _wplayerui (`/Game/Lee/GameMode/MyHUD.WPlayerUI` _asmy_hud))
  (bind _output_get (set `self.Player UI` _wplayerui))
  (`Widget.SetVisibility` (`/Game/Lee/UI/W_PlayerUI.TextBlock` _output_get) "Visible")
  (set `/Game/Lee/UI/W_PlayerUI.Text` "잠겨 있다" _wplayerui)
  (`KismetSystemLibrary.K2_SetTimerDelegate` (`|CreateDelegate` :!event `SetHidden`) 2.0))

(event `SetHidden`
  (`Widget.SetVisibility` (`/Game/Lee/UI/W_PlayerUI.TextBlock` (`self.Player UI`)) "Hidden"))

(fn `UserConstructionScript`)